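; RakNetRP actor that starts and disconnects the RakNet RP client and visualizes server boundaries as floors.
; Boundary events spawn Floor_Blueprint actors tagged with server Rank and tinted through dynamic materials, and delete boxes by Rank.
; F sends a test spawn RPC from the camera, swapping Y/Z and rescaling between Unreal and server coordinates.
; ConnectFromCmd connects to numbered IP host:port options; the position-response binding never runs.
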(event `self.ReceiveBeginPlay`
  (`|ExecutionSequence`
    (:`then_0`
      (`self.EnableInput` (`GameplayStatics.GetPlayerController` 0)))
    (:`then_1`
      (`KismetSystemLibrary.Delay` 1.0)
      (`self.RPStartup`))
    (:`then_2`
      (set `self.BigScale` (100000.0 100000.0 1.0)))
    (:`then_3`
      (`self.GenrateColor`)
      (`KismetSystemLibrary.PrintString` "Run"))))

(event `self.ReceiveEndPlay`
  (params (EndPlayReason :type "EEndPlayReason Enum" :default "Destroyed"))
  (`self.RPDisconnect`))

(event `OnReceiveResponse_Event_0` :!signature `self.OnReceiveResponse`
  (params (receivedVector :type "Vector Structure"))
  (`SceneComponent.K2_SetWorldLocation` (`self.DefaultSceneRoot`) receivedVector false true))

(event `Key|F`
  (params (Key :type "Key Structure"))
  (bind _returnvalue (`GameplayStatics.GetPlayerCameraManager` 0))
  (:`Pressed`
    (`KismetSystemLibrary.PrintString` "RPrpc Test called")
    (`self.RPrpcSpawn` (/ (`KismetMathLibrary.MakeVector` (.x (`PlayerCameraManager.GetCameraLocation` _returnvalue)) (.z (`PlayerCameraManager.GetCameraLocation` _returnvalue)) (.y (`PlayerCameraManager.GetCameraLocation` _returnvalue))) 50.0) (`KismetMathLibrary.MakeVector` (.x (`KismetMathLibrary.GetForwardVector` (`PlayerCameraManager.GetCameraRotation` _returnvalue))) (.z (`KismetMathLibrary.GetForwardVector` (`PlayerCameraManager.GetCameraRotation` _returnvalue))) (.y (`KismetMathLibrary.GetForwardVector` (`PlayerCameraManager.GetCameraRotation` _returnvalue)))))))

(event `self.CreateBoundaryBox`
  (params (rank :type Integer) (pos :type "Vector Structure") (size :type "Vector Structure"))
  (bind _randomfloorcolor (`self.RandomFloorColor`))
  (bind _randomfloorcolor_2 (`self.RandomFloorColor`))
  (`KismetSystemLibrary.PrintString` (`KismetStringLibrary.Concat_StrStr` (`KismetStringLibrary.Conv_VectorToString` pos) (`KismetStringLibrary.Conv_VectorToString` size)))
  (bind _returnvalue (`|SpawnActorFromClass` "/Game/Blueprints/Floor_Blueprint.Floor_Blueprint_C" (`KismetMathLibrary.MakeTransform` (* (`KismetMathLibrary.MakeVector` (.x pos) (.z pos)) 50.0) (struct) (`KismetMathLibrary.MakeVector` (.x (/ size 2.0)) (.z (/ size 2.0)) 1.0)) "AlwaysSpawn" "OverrideRootScale" null null))
  (bind _returnvalue_2 (`PrimitiveComponent.CreateDynamicMaterialInstance` (`StaticMeshActor.StaticMeshComponent` _returnvalue) 0 "/Game/Materials/M_Server_Floor.M_Server_Floor"))
  (switch `int` rank
    (:`Default`
      (set `self.Colour` (`KismetMathLibrary.RandomUnitVectorInConeInRadians` (0.5 0.5 0.5) 3.142)))
    (:`0`
      (`self.SetColor` 0)
      (`KismetSystemLibrary.PrintString` (`KismetStringLibrary.Conv_ColorToString` _randomfloorcolor) true true (struct :`G` 0.66 :`B` 1.0 :`A` 1.0) 15.0)
      (set `self.Colour` (`KismetMathLibrary.Conv_LinearColorToVector` _randomfloorcolor)))
    (:`1`
      (`self.SetColor` 1)
      (`KismetSystemLibrary.PrintString` (`KismetStringLibrary.Conv_ColorToString` _randomfloorcolor_2) true true (struct :`G` 0.66 :`B` 1.0 :`A` 1.0) 15.0)
      (set `self.Colour` (`KismetMathLibrary.Conv_LinearColorToVector` _randomfloorcolor_2)))
    (:`2`
      (`self.SetColor` 2)
      (set `self.Colour` (`KismetMathLibrary.Conv_LinearColorToVector` (`self.RandomFloorColor`))))
    (:`3`
      (`self.SetColor` rank)
      (set `self.Colour` (`KismetMathLibrary.Conv_LinearColorToVector` (`self.RandomFloorColor`)))))
  (`MaterialInstanceDynamic.SetVectorParameterValue` _returnvalue_2 "Colour" (`KismetMathLibrary.Conv_VectorToLinearColor` (`self.Colour`)))
  (set `/Game/Blueprints/Floor_Blueprint.rank` rank _returnvalue))

(event `self.CreateBoundaryPlane`
  (params (rank :type Integer) (pos :type "Vector Structure") (normal :type "Vector Structure"))
  (bind _returnvalue (`|SpawnActorFromClass` "/Game/Blueprints/Floor_Blueprint.Floor_Blueprint_C" (`KismetMathLibrary.MakeTransform` (+ (`KismetMathLibrary.MakeVector` (.x pos) (.z pos) (.y pos)) (* (* (0.0 1.0 0.0) (`self.BigScale`)) 50.0)) (struct) (`self.BigScale`)) "AlwaysSpawn" "OverrideRootScale" null null))
  (bind _returnvalue_2 (`PrimitiveComponent.CreateDynamicMaterialInstance` (`StaticMeshActor.StaticMeshComponent` _returnvalue) 0 "/Game/Materials/M_Server_Floor.M_Server_Floor"))
  (`MaterialInstanceDynamic.SetVectorParameterValue` _returnvalue_2 "Colour" (`KismetMathLibrary.Conv_VectorToLinearColor` (`KismetMathLibrary.RandomUnitVectorInConeInRadians` (0.5 0.5 0.5) 3.142)))
  (set `/Game/Blueprints/Floor_Blueprint.rank` rank _returnvalue))

(event `self.DeleteBoundaryBox`
  (params (rank :type Integer))
  (bind _outactors (`GameplayStatics.GetAllActorsOfClass` "/Game/Blueprints/Floor_Blueprint.Floor_Blueprint_C"))
  (for _array_element _outactors
    (if (== rank (`/Game/Blueprints/Floor_Blueprint.rank` _array_element))
      (`self.K2_DestroyActor` _array_element))))

(fn `ConnectFromCmd`
  (params (Options :type String))
  (bind _returnvalue (`KismetStringLibrary.Concat_StrStr` "IP" (`KismetStringLibrary.Conv_IntToString` (`self.IPCounter`))))
  (bind _returnvalue_2 (`GameplayStatics.ParseOption` Options _returnvalue))
  (bind (_lefts _rights) (`KismetStringLibrary.Split` _returnvalue_2 ":"))
  (`KismetSystemLibrary.PrintString` Options)
  (bind _returnvalue_3 (`KismetSystemLibrary.GetCommandLine`))
  (`KismetSystemLibrary.PrintString` _returnvalue_3)
  (set `self.IPCounter` 1)
  (`KismetSystemLibrary.PrintString` _returnvalue true true (struct :`G` 0.66 :`B` 1.0 :`A` 1.0) 120.0)
  (while (`GameplayStatics.HasOption` Options _returnvalue)
    (`KismetSystemLibrary.PrintString` _returnvalue_2 true true (struct :`G` 0.66 :`B` 1.0 :`A` 1.0) 120.0)
    (`self.RPConnect` _lefts (`KismetStringLibrary.Conv_StringToInt` _rights))
    (`/Engine/EditorBlueprintResources/StandardMacros.IncrementInt` (`self.IPCounter`))))

(fn `UserConstructionScript`)