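; LevelChanger is a Blueprint that opens the level menu when the P key is pressed.
; It creates a LevelMenuBP widget for the first player, passes it a reference to itself, adds it to the viewport, then shows the cursor and switches to UI-only input.
; A Pressed flag blocks repeat opening and is never cleared within this Blueprint.
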(event `Key|P`
  (params (Key :type "Key Structure"))
  (bind _returnvalue (`GameplayStatics.GetPlayerController` 0))
  (:`Pressed`
    (if (not (`self.pressed`))
      (bind _returnvalue_2 (`|CreateWidget` "/Game/Blueprints/LevelMenu/LevelMenuBP.LevelMenuBP_C" _returnvalue))
      (set `/Game/Blueprints/LevelMenu/LevelMenuBP.LevelChanger` self _returnvalue_2)
      (`UserWidget.AddToViewport` _returnvalue_2 0)
      (set `PlayerController.bShowMouseCursor` true _returnvalue)
      (`WidgetBlueprintLibrary.SetInputMode_UIOnlyEx` _returnvalue _returnvalue_2)
      (set `self.pressed` true)
      (set `/Game/Blueprints/LevelMenu/LevelMenuBP.LevelChanger` self _returnvalue_2))))

(fn `UserConstructionScript`)